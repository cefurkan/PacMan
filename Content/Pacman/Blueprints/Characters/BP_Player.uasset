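; Player Pac-Man character that keeps moving in the last pressed direction and animates its gobbling mouth.
; MoveForward and MoveRight axis input past a threshold latches one direction flag and applies movement immediately.
; Once AllowedToMove is set, Tick repeats that movement along yaw-only control-rotation axes.
; While ShouldPlayerGobble is true, Tick also toggles PlayerOpen and PlayerClosed visibility after a short Delay.
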(event `self.ReceiveTick`
  (params (DeltaSeconds :type "Float (single-precision)"))
  (if (`self.bAllowedToMove?`)
    (`|ExecutionSequence`
      (:`then_0`
        ;[0 1 0.04933] Player Gobble Anımatıon
        (if (`self.bShouldPlayerGobble?`)
          (`KismetSystemLibrary.Delay` 0.05)
          (`/Engine/EditorBlueprintResources/StandardMacros.FlipFlop`
            (:`A`
              _)
            (:`B`
              _))
          (`SceneComponent.ToggleVisibility` (`self.Player_Open`) false)
          (`SceneComponent.ToggleVisibility` (`self.Player_Closed`) false)))
      (:`then_1`
        (if (`self.bGoingUp?`)
          ;[0 1 0.04933] Player Move Up/Down
          (`self.AddMovementInput` (`KismetMathLibrary.GetRightVector` (`KismetMathLibrary.MakeRotator` 0.0 0.0 (.yaw (`self.GetControlRotation`)))) (stale `InputAxis|MoveRight` _output_get) :!label _label)
          (elif (`self.bGoingUpDown?`)
            (`self.AddMovementInput` (`KismetMathLibrary.GetRightVector` (`KismetMathLibrary.MakeRotator` 0.0 0.0 (.yaw (`self.GetControlRotation`)))) (stale `InputAxis|MoveRight` _output_get_2) :!label _label_2)
            (elif (`self.bGoingLeft?`)
              ;[0 1 0.04933] Player Move Right/Left
              (`self.AddMovementInput` (`KismetMathLibrary.GetForwardVector` (`KismetMathLibrary.MakeRotator` 0.0 0.0 (.yaw (`self.GetControlRotation`)))) (stale `InputAxis|MoveForward` _output_get_2) :!label _label_3)
              (elif (`self.bGoingRight?`)
                (`self.AddMovementInput` (`KismetMathLibrary.GetForwardVector` (`KismetMathLibrary.MakeRotator` 0.0 0.0 (.yaw (`self.GetControlRotation`)))) (stale `InputAxis|MoveForward` _output_get) :!label _label_4)))))))))

(event `InputAxis|MoveForward` :overrideparent false
  (params (AxisValue :type "Float (single-precision)"))
  ;[0 1 0.04933] Player Move Right/Left
  (if (>= AxisValue 0.7)
    (set `self.bGoingUpDown?` false)
    (set `self.bGoingUp?` false)
    (set `self.bGoingLeft?` false)
    (set `self.bGoingRight?` true)
    (bind _output_get (set `self.InputForward` 1.0))
    (goto _label_4)
    (elif (<= AxisValue -0.7)
      (set `self.bGoingUpDown?` false)
      (set `self.bGoingUp?` false)
      (set `self.bGoingRight?` false)
      (set `self.bGoingLeft?` true)
      (bind _output_get_2 (set `self.InputForward` -1.0))
      (goto _label_3))))

(event `InputAxis|MoveRight` :overrideparent false
  (params (AxisValue :type "Float (single-precision)"))
  ;[0 1 0.04933] Player Move Up/Down
  (if (>= AxisValue 0.7)
    (set `self.bGoingUpDown?` false)
    (set `self.bGoingLeft?` false)
    (set `self.bGoingRight?` false)
    (set `self.bGoingUp?` true)
    (bind _output_get (set `self.InputRight` 1.0))
    (goto _label)
    (elif (<= AxisValue -0.7)
      (set `self.bGoingUp?` false)
      (set `self.bGoingRight?` false)
      (set `self.bGoingLeft?` false)
      (set `self.bGoingUpDown?` true)
      (bind _output_get_2 (set `self.InputRight` -1.0))
      (goto _label_2))))

(fn `UserConstructionScript`)