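; BP_Player2 is a Pac-Man-style player character that keeps moving in its last input direction and handles speed boosts, death and respawn.
; Axis input latches one of four direction flags that Tick turns into yaw-relative movement, while toggling open and closed meshes animates gobbling.
; SPEEDBOOST temporarily changes speed, material and effects.
; BP_Enemy_Parent's KilledPlayer dispatcher cancels boosts, stops control and plays spin, sound, particles and camera shake before respawning.
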(event `self.ReceiveTick`
  (params (DeltaSeconds :type "Float (single-precision)"))
  (if (`self.bAllowedToMove?`)
    (`|ExecutionSequence`
      (:`then_0`
        ;[0 1 0.04933] Player Gobble Anımatıon
        (if (`self.bShouldPlayerGobble?`)
          (`KismetSystemLibrary.Delay` 0.05)
          (`/Engine/EditorBlueprintResources/StandardMacros.FlipFlop`
            (:`A`
              _)
            (:`B`
              _))
          (`SceneComponent.ToggleVisibility` (`self.Player_Open`) false)
          (`SceneComponent.ToggleVisibility` (`self.Player_Closed`) false)))
      (:`then_1`
        (if (`self.bGoingUp?`)
          ;[0 1 0.04933] Player Move Up/Down
          (`self.AddMovementInput` (`KismetMathLibrary.GetRightVector` (`KismetMathLibrary.MakeRotator` 0.0 0.0 (.yaw (`self.GetControlRotation`)))) (stale `InputAxis|MoveRight` _output_get) :!label _label)
          (elif (`self.bGoingUpDown?`)
            (`self.AddMovementInput` (`KismetMathLibrary.GetRightVector` (`KismetMathLibrary.MakeRotator` 0.0 0.0 (.yaw (`self.GetControlRotation`)))) (stale `InputAxis|MoveRight` _output_get_2) :!label _label_2)
            (elif (`self.bGoingLeft?`)
              ;[0 1 0.04933] Player Move Right/Left
              (`self.AddMovementInput` (`KismetMathLibrary.GetForwardVector` (`KismetMathLibrary.MakeRotator` 0.0 0.0 (.yaw (`self.GetControlRotation`)))) (stale `InputAxis|MoveForward` _output_get_2) :!label _label_3)
              (elif (`self.bGoingRight?`)
                (`self.AddMovementInput` (`KismetMathLibrary.GetForwardVector` (`KismetMathLibrary.MakeRotator` 0.0 0.0 (.yaw (`self.GetControlRotation`)))) (stale `InputAxis|MoveForward` _output_get) :!label _label_4)))))))))

(event `InputAxis|MoveForward` :overrideparent false
  (params (AxisValue :type "Float (single-precision)"))
  ;[0 1 0.04933] Player Move Right/Left
  (if (>= AxisValue 0.7)
    (set `self.bGoingUpDown?` false)
    (set `self.bGoingUp?` false)
    (set `self.bGoingLeft?` false)
    (set `self.bGoingRight?` true)
    (bind _output_get (set `self.InputForward` 1.0))
    (goto _label_4)
    (elif (<= AxisValue -0.7)
      (set `self.bGoingUpDown?` false)
      (set `self.bGoingUp?` false)
      (set `self.bGoingRight?` false)
      (set `self.bGoingLeft?` true)
      (bind _output_get_2 (set `self.InputForward` -1.0))
      (goto _label_3))))

(event `InputAxis|MoveRight` :overrideparent false
  (params (AxisValue :type "Float (single-precision)"))
  ;[0 1 0.04933] Player Move Up/Down
  (if (>= AxisValue 0.7)
    (set `self.bGoingUpDown?` false)
    (set `self.bGoingLeft?` false)
    (set `self.bGoingRight?` false)
    (set `self.bGoingUp?` true)
    (bind _output_get (set `self.InputRight` 1.0))
    (goto _label)
    (elif (<= AxisValue -0.7)
      (set `self.bGoingUp?` false)
      (set `self.bGoingRight?` false)
      (set `self.bGoingLeft?` false)
      (set `self.bGoingUpDown?` true)
      (bind _output_get_2 (set `self.InputRight` -1.0))
      (goto _label_2))))

(event `UNDO SPEED BOOST`
  ;[1 1 1] Player Was Killed!
  ;[0 1 0.04933] Speed Boost
  (set `self.bIsBoosted?` false :!label _label_5)
  (set `CharacterMovementComponent.MaxWalkSpeed` (`self.PlayerRegularSpeed`) (`self.CharacterMovement`))
  (`PrimitiveComponent.SetMaterial` (`self.Player_Closed`) 0 "/Game/Pacman/Materials/M_Base_Inst_Player.M_Base_Inst_Player")
  (`PrimitiveComponent.SetMaterial` (`self.Player_Open`) 0 "/Game/Pacman/Materials/M_Base_Inst_Player.M_Base_Inst_Player")
  (`ActorComponent.Deactivate` (`self.VFX_PowerUpSpeed`))
  (`ActorComponent.Deactivate` (`self.SFX_PowerUpSpeed`)))

(event `SPEED BOOST`
  ;[0 1 0.04933] Speed Boost
  (set `self.bIsBoosted?` true)
  (set `CharacterMovementComponent.MaxWalkSpeed` (`self.PlayerBoostedSpeed`) (`self.CharacterMovement`))
  (`PrimitiveComponent.SetMaterial` (`self.Player_Closed`) 0 "/Game/Pacman/Materials/M_Base_Inst_Fruit_Cherries.M_Base_Inst_Fruit_Cherries")
  (`PrimitiveComponent.SetMaterial` (`self.Player_Open`) 0 "/Game/Pacman/Materials/M_Base_Inst_Fruit_Cherries.M_Base_Inst_Fruit_Cherries")
  (`ActorComponent.Activate` (`self.VFX_PowerUpSpeed`) false)
  (`ActorComponent.Activate` (`self.SFX_PowerUpSpeed`) false)
  (`KismetSystemLibrary.Delay` 6.0)
  (goto _label_5))

(event `RESPAWN PLAYER`
  ;[0 1 0.04933] Player Respawn Script
  (`KismetSystemLibrary.Delay` 1.5)
  (`self.K2_SetActorLocationAndRotation` (`self.PlayerSpawnLocale`))
  (`GameplayStatics.SpawnEmitterAtLocation` "/Game/Pacman/Particles/P_Respawn_Player.P_Respawn_Player" (`SceneComponent.K2_GetComponentLocation` (`self.CapsuleComponent`)))
  (`KismetSystemLibrary.Delay` 1.0)
  (`self.SetActorHiddenInGame` false)
  (`KismetSystemLibrary.Delay` 2.5)
  (`self.EnableInput` (`GameplayStatics.GetPlayerController` 0))
  (set `self.bShouldPlayerGobble?` true)
  (set `self.bGoingRight?` true)
  (set `self.InputForward` 1.0)
  (set `CharacterMovementComponent.MaxWalkSpeed` (`self.PlayerRegularSpeed`) (`self.CharacterMovement`)))

(event `LISTEN FOR PLAYER KILL`
  ;[0 1 0.04933] Listen out for "KilledPlayer" Event Dispatcher
  (add `/Game/Pacman/Blueprints/Characters/BP_Enemy_Parent.KilledPlayer` (`self.Enemy Parent`) (delegate `KilledPlayer_Event_0`)))

(event `KilledPlayer_Event_0`
  ;[0 1 0.04933] Listen out for "KilledPlayer" Event Dispatcher
  (`|ExecutionSequence`
    (:`then_0`
      ;[0 1 0.04933] Kill Speed Boost FX (if boosted)
      (`self.UNDO SPEED BOOST`))
    (:`then_1`
      ;[0 1 0.04933] Stop Input, Gobbling, Navigation
      (`self.DisableInput` (`GameplayStatics.GetPlayerController` 0))
      (set `self.bShouldPlayerGobble?` false)
      (set `self.bGoingRight?` false)
      (set `self.bGoingUp?` false)
      (set `self.bGoingLeft?` false)
      (set `self.bGoingUpDown?` false)
      (set `self.InputForward` 0.0)
      (set `self.InputForward` 0.0)
      (set `CharacterMovementComponent.MaxWalkSpeed` 0.0 (`self.CharacterMovement`)))
    (:`then_2`
      ;[0 1 0.04933] Player Death FX
      (`GameplayStatics.PlaySound2D` "/Game/Pacman/Audio/SFX_Death_Cue.SFX_Death_Cue" 1.0 1.0 0.0 null null)
      (`KismetSystemLibrary.Delay` 1.75)
      (`GameplayStatics.SpawnEmitterAtLocation` "/Game/Pacman/Particles/P_Death.P_Death" (`self.K2_GetActorLocation`) (struct) (3.0 3.0 3.0))
      (`self.SetActorHiddenInGame` true)
      ;[0 1 0.04933] Call To Respawn
      (`self.RESPAWN PLAYER`))
    (:`then_3`
      ;[0 1 0.04933] Player Death Animation
      (bind (_direction _player_rotation) (`Timeline|Death Spin` :!via `PlayFromStart`)
        (:`Update`
          (`SceneComponent.K2_SetRelativeRotation` (`self.CapsuleComponent`) (`KismetMathLibrary.MakeRotator` 0.0 0.0 _player_rotation) false false))
        (:`Finished`
          ;[0 1 0.04933] Death Cam Shake
          (`GameplayStatics.PlayWorldCameraShake` "/Game/Pacman/Blueprints/Misc/BP_DeathCamShake.BP_DeathCamShake_C" (0.0 230.0 3000.0) 0.0 1000.0))))
    (:`then_4`
      ;[0 1 0.04933] Ensure Player Mouth Open on Death
      (`KismetSystemLibrary.Delay` 0.1)
      (`SceneComponent.SetVisibility` (`self.Player_Open`) true false)
      (`SceneComponent.SetVisibility` (`self.Player_Closed`) false false))))

(event `self.ReceiveBeginPlay`
  (`|ExecutionSequence`
    (:`then_0`
      ;[0 1 0.04933] Reference to Enemy Parent
      (bind _outactors (`GameplayStatics.GetAllActorsOfClass` "/Game/Pacman/Blueprints/Characters/BP_Enemy_Parent.BP_Enemy_Parent_C"))
      (set `self.Enemy Parent` _outactors)
      ;[0 1 0.04933] Initializes listening of Player Kill Event
      (`self.LISTEN FOR PLAYER KILL`))))

(fn `UserConstructionScript`)