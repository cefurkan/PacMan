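; Gameplay game mode for a Pac-Man game that handles level intro, bonus pickup spawning and level completion.
; BeginPlay tallies regular and power pellets, blends to a spawned gameplay camera while player input is disabled, and after a random delay spawns one random fruit or speed power-up.
; The ATEPELLET event counts pellets down; at zero it blocks bonus spawning, prints end of level and stops the player.
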(event `ATE PELLET`
  (bind _playerref (`self.PlayerRef`))
  ;[0 1 0.04933] Level Completion Check(runs script whenever a pellet is eaten)
  (bind _result (`/Engine/EditorBlueprintResources/StandardMacros.DecrementInt` (`self.TotalPellets`)) ; subtract 1 pellet
    (:`  `
      (bind _output_get (set `self.TotalPellets` _result))
      (if (<= _output_get 0)
        (set `self.bGoodieSpawnOK` false)
        (`|ExecutionSequence`
          (:`then_0`
            (`KismetSystemLibrary.PrintString` "End of Level"))
          (:`then_1`
            ;[0 1 0.04933] Stop Player Nav
            (`self.DisableInput` (`GameplayStatics.GetPlayerCharacter` 0) (`GameplayStatics.GetPlayerController` 0))
            (set `CharacterMovementComponent.MaxWalkSpeed` 0.0 (`Character.CharacterMovement` _playerref))
            (set `/Game/Pacman/Blueprints/Characters/BP_Player2.bShouldPlayerGobble?` false _playerref)))))))

(event `self.ReceiveBeginPlay`
  (bind _returnvalue (`GameplayStatics.GetPlayerCharacter` 0))
  (`|ExecutionSequence`
    (:`then_0`
      ;[0 1 0.04933] ReferenceToPlayer
      (bind _asbp_player_2 (cast `/Game/Pacman/Blueprints/Characters/BP_Player2` (`GameplayStatics.GetPlayerCharacter` 0)))
      (set `self.PlayerRef` _asbp_player_2))
    (:`then_1`
      ;[0 1 0.04933] Tally Total Pallets existing in level
      (bind _outactors (`GameplayStatics.GetAllActorsOfClass` "/Game/Pacman/Blueprints/Pickups/BP_Pellet.BP_Pellet_C"))
      (bind _output_get (set `self.TotalRegularPellets` (`KismetArrayLibrary.Array_Length` _outactors))))
    (:`then_2`
      (bind _outactors_2 (`GameplayStatics.GetAllActorsOfClass` "/Game/Pacman/Blueprints/Pickups/BP_PowerPellet.BP_PowerPellet_C"))
      (bind _output_get_2 (set `self.TotalPowerPellets` (`KismetArrayLibrary.Array_Length` _outactors_2)))
      (bind _output_get_3 (set `self.TotalPellets` (+ _output_get _output_get_2)))
      (`KismetSystemLibrary.PrintString` (`KismetStringLibrary.Conv_IntToString` _output_get_3) true true (struct :`G` 0.66 :`B` 1.0 :`A` 1.0) 5.0))
    (:`then_3`
      ;[1 0.9385 0.3582] Gameplay Camera
      (`self.DisableInput` (`GameplayStatics.GetPlayerCharacter` 0) (`GameplayStatics.GetPlayerController` 0))
      (bind _returnvalue_2 (`|SpawnActorFromClass` "/Script/Engine.CameraActor" (`KismetMathLibrary.MakeTransform` (`self.CamGameplay_Loc`) (`self.CamGameplay_Rot`)) "Undefined" "OverrideRootScale" null null))
      (`PlayerController.SetViewTargetWithBlend` (`GameplayStatics.GetPlayerController` 0) _returnvalue_2 3.0 "VTBlend_Linear" 0.0 false)
      (`KismetSystemLibrary.Delay` 3.0)
      (`self.EnableInput` _returnvalue (`GameplayStatics.GetPlayerController` 0))
      (bind _asbp_player_2_2 (cast `/Game/Pacman/Blueprints/Characters/BP_Player2` _returnvalue)))
    (:`then_5`
      ;[0 1 0.04933] Fruit Power Up Spawn
      (`KismetSystemLibrary.Delay` (`KismetMathLibrary.RandomFloatInRange` 5.0 10.0))
      (if (`self.bGoodieSpawnOK`)
        (bind _output_get_4 (set `self.GoodieSpawnLocales` (`|MakeArray` (`self.GoodieSpawn_01`) (`self.GoodieSpawn_02`))))
        (switch `int` (`KismetMathLibrary.RandomIntegerInRange` 0 2)
          (:`0`
            (bind _returnvalue_3 (`KismetMathLibrary.Conv_VectorToTransform` (`|GetArrayItem` _output_get_4 (`KismetMathLibrary.RandomIntegerInRange` 0 (- (`KismetArrayLibrary.Array_Length` _output_get_4) 1)))))
            (`|SpawnActorFromClass` "/Game/Pacman/Blueprints/Pickups/BP_Food_Cherry.BP_Food_Cherry_C" _returnvalue_3 "Undefined" "OverrideRootScale" null null))
          (:`1`
            (`|SpawnActorFromClass` "/Game/Pacman/Blueprints/Pickups/BP_Food_Orange.BP_Food_Orange_C" _returnvalue_3 "Undefined" "OverrideRootScale" null null))
          (:`2`
            (`|SpawnActorFromClass` "/Game/Pacman/Blueprints/Pickups/BP_PowerUp_Speed.BP_PowerUp_Speed_C" _returnvalue_3 "Undefined" "OverrideRootScale" null null)))))))

(fn `UserConstructionScript`)